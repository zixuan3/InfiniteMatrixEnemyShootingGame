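; BP_Tunnel is an endless-runner tunnel segment with a rotating holed wall, health pack and enemy.
; Randomize functions vary the wall mesh and roll, enemy look and position, and health pack presence and offset.
; Overlaps apply healing, damage, death and score changes to BP_Player, and fireballs destroy the enemy for a point.
; When the player exits TriggerZone, TunnelSpawner spawns the next segment, this one destroys itself and the player scores.
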(event OnComponentBeginOverlap(HealthPack)
  (params (OverlappedComponent :type Primitive%20Component%20Object%20Reference) (OtherActor :type Actor%20Object%20Reference) (OtherComp :type Primitive%20Component%20Object%20Reference) (OtherBodyIndex :type Integer) (bFromSweep :type Boolean) (SweepResult :type Hit%20Result%20Structure%20%28by%20ref%29))
  (bind _asbp_player (Utilities|Casting|CastToBP_Player OtherActor))
  (Variables|/Game/InfiniteMatrix/Blueprints/BP_Player.BP_Player_C|SetCurrentHealth _asbp_player (Math|Float|Min(Float) (Variables|/Game/InfiniteMatrix/Blueprints/BP_Player.BP_Player_C|GetMaxHealth _asbp_player) (+ (Variables|/Game/InfiniteMatrix/Blueprints/BP_Player.BP_Player_C|GetCurrentHealth _asbp_player) 2e+01)))
  (Components|DestroyComponent (Variables|Default|GetHealthPack)))

(event OnComponentBeginOverlap(WallMesh)
  (params (OverlappedComponent :type Primitive%20Component%20Object%20Reference) (OtherActor :type Actor%20Object%20Reference) (OtherComp :type Primitive%20Component%20Object%20Reference) (OtherBodyIndex :type Integer) (bFromSweep :type Boolean) (SweepResult :type Hit%20Result%20Structure%20%28by%20ref%29))
  (bind _asbp_player (Utilities|Casting|CastToBP_Player OtherActor))
  (Math|Float|CompareFloat (- (Variables|/Game/InfiniteMatrix/Blueprints/BP_Player.BP_Player_C|GetCurrentHealth _asbp_player) 1e+01) 0.0
    (:>
      (Variables|/Game/InfiniteMatrix/Blueprints/BP_Player.BP_Player_C|SetCurrentHealth _asbp_player (- (Variables|/Game/InfiniteMatrix/Blueprints/BP_Player.BP_Player_C|GetCurrentHealth _asbp_player) 1e+01)))
    (:==
      (Variables|/Game/InfiniteMatrix/Blueprints/BP_Player.BP_Player_C|SetCurrentHealth _asbp_player (- (Variables|/Game/InfiniteMatrix/Blueprints/BP_Player.BP_Player_C|GetCurrentHealth _asbp_player) 1e+01))
      (Variables|/Game/InfiniteMatrix/Blueprints/BP_Player.BP_Player_C|SetIsDead _asbp_player true :!label _label)
      (Default|DisplayRestart _asbp_player))
    (:<
      (goto _label))))

(event OnComponentEndOverlap(TriggerZone)
  (params (OverlappedComponent :type Primitive%20Component%20Object%20Reference) (OtherActor :type Actor%20Object%20Reference) (OtherComp :type Primitive%20Component%20Object%20Reference) (OtherBodyIndex :type Integer))
  (bind _asbp_player (Utilities|Casting|CastToBP_Player OtherActor))
  (Default|SpawnTunnelatSpawnPoint (Variables|Default|GetTunnelSpawner))
  (Actor|DestroyActor)
  (Default|AddScore _asbp_player 1))

(event OnComponentEndOverlap(WallMesh)
  (params (OverlappedComponent :type Primitive%20Component%20Object%20Reference) (OtherActor :type Actor%20Object%20Reference) (OtherComp :type Primitive%20Component%20Object%20Reference) (OtherBodyIndex :type Integer))
  (bind _asbp_player (Utilities|Casting|CastToBP_Player OtherActor))
  (Default|MinusScore _asbp_player 1))

(event OnComponentBeginOverlap(Enemy)
  (params (OverlappedComponent :type Primitive%20Component%20Object%20Reference) (OtherActor :type Actor%20Object%20Reference) (OtherComp :type Primitive%20Component%20Object%20Reference) (OtherBodyIndex :type Integer) (bFromSweep :type Boolean) (SweepResult :type Hit%20Result%20Structure%20%28by%20ref%29))
  (bind _outactors (Actor|GetAllActorsOfClass "/Game/InfiniteMatrix/Blueprints/BP_Player.BP_Player_C"))
  (bind _asbp_player (Utilities|Casting|CastToBP_Player OtherActor)
    (:then
      (Default|MinusScore _asbp_player 1)
      (Math|Float|CompareFloat (- (Variables|/Game/InfiniteMatrix/Blueprints/BP_Player.BP_Player_C|GetCurrentHealth _asbp_player) 1e+01) 0.0
        (:>
          (Variables|/Game/InfiniteMatrix/Blueprints/BP_Player.BP_Player_C|SetCurrentHealth _asbp_player (- (Variables|/Game/InfiniteMatrix/Blueprints/BP_Player.BP_Player_C|GetCurrentHealth _asbp_player) 1e+01))
          (Components|DestroyComponent (Variables|Default|GetEnemy)))
        (:==
          (Variables|/Game/InfiniteMatrix/Blueprints/BP_Player.BP_Player_C|SetCurrentHealth _asbp_player (- (Variables|/Game/InfiniteMatrix/Blueprints/BP_Player.BP_Player_C|GetCurrentHealth _asbp_player) 1e+01))
          (Variables|/Game/InfiniteMatrix/Blueprints/BP_Player.BP_Player_C|SetIsDead _asbp_player true :!label _label)
          (Default|DisplayRestart _asbp_player))
        (:<
          (goto _label))))
    (:CastFailed
      (Utilities|Casting|CastToFireball_BP_Proj OtherActor)
      (Default|AddScore (Utilities|Array|Get(acopy) _outactors) 1)
      (Components|DestroyComponent (Variables|Default|GetEnemy)))))

(event EventBeginPlay)

(event EventTick
  (params (DeltaSeconds :type Float%20%28single-precision%29))
  (Transformation|AddLocalRotation (Variables|Default|GetWallMesh) (Math|Rotator|MakeRotator (* DeltaSeconds (Variables|Default|GetRotateSpeed)) 0.0 0.0) false false))

(fn ConstructionScript)

(fn RandomizeWall
  (Components|StaticMesh|SetStaticMesh (Variables|Default|GetWallMesh) (Utilities|Select :Index (Math|Random|RandomIntegerinRange 0 3) :Option%200 "/Game/InfiniteMatrix/Meshes/SM_Hole_01.SM_Hole_01" :Option%201 "/Game/InfiniteMatrix/Meshes/SM_Hole_02.SM_Hole_02" :Option%202 "/Game/InfiniteMatrix/Meshes/SM_Hole_03.SM_Hole_03" :Option%203 "/Game/InfiniteMatrix/Meshes/SM_Hole_04.SM_Hole_04"))
  (Transformation|AddLocalRotation (Variables|Default|GetWallMesh) (Math|Rotator|MakeRotator (Math|Random|RandomFloatinRange 0.0 3.6e+02) 0.0 0.0) false false))

(fn RandomizeHealthPack
  (bind _healthpack (Variables|Default|GetHealthPack))
  (bind _returnvalue (Transformation|GetWorldLocation _healthpack))
  (if (Math|Random|RandomBoolwithWeight 0.25)
    (Transformation|SetWorldLocation _healthpack (Math|Vector|MakeVector (+ (Math|Random|RandomFloatinRange -3e+02 3e+02) (.x _returnvalue)) (+ (Math|Random|RandomFloatinRange -3e+02 3e+02) (.y _returnvalue)) (+ (Math|Random|RandomFloatinRange -3e+02 3e+02) (.z _returnvalue))) false true)
    (else
      (Components|DestroyComponent _healthpack))))

(fn RandomizeEnemy
  (bind _enemy (Variables|Default|GetEnemy))
  (bind _returnvalue (Transformation|GetWorldLocation _enemy))
  (Components|StaticMesh|SetStaticMesh _enemy (Utilities|Select :Index (Math|Random|RandomIntegerinRange 0 3) :Option%200 "/Game/Meshes/SM_Corpse.SM_Corpse" :Option%201 "/Game/Meshes/SM_MERGED_Archor_Bow.SM_MERGED_Archor_Bow" :Option%202 "/Game/Meshes/SM_MERGED_Charger_Helmet.SM_MERGED_Charger_Helmet" :Option%203 "/Game/Meshes/SM_Corpse_Melee.SM_Corpse_Melee"))
  (Transformation|SetWorldLocation _enemy (Math|Vector|MakeVector (.x _returnvalue) (+ (Math|Random|RandomFloatinRange -3e+02 2e+02) (.y _returnvalue)) (+ (Math|Random|RandomFloatinRange -2e+02 2e+02) (.z _returnvalue))) false true))